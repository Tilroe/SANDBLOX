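; Player controller for a multiplayer block-building game with chat, spectator toggling, and widgets for block color, shape and pause.
; Each tick, a mouse trace snaps a rotatable preview block onto Stud components for placement.
; SR_ events store placed blocks in the game instance and relay placement, deletion and chat to each controller's OC_ events; joining replays saved blocks.
; Deletion re-traces on each client, running first on the initiator.
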(event Custom|OC_Update_Chat
  (params (PlayerName :type Text) (ChatMessage :type Text))
  ;[0.05098 0.05098 0.05098] ChatBox
  (bind _wb_chatpanel (Variables|Default|GetWB_ChatPanel)
    (:then
      (Default|UpdateChat _wb_chatpanel PlayerName ChatMessage))
    (:else)))

(event Custom|SR_SpawnPlayer
  (params (Pawn%20Class :type Pawn%20Class%20Reference))
  ;[1 1 1] Spawn PlayerPawn
  (bind _asgm_master (Utilities|Casting|CastToGM_Master (Game|GetGameMode)))
  (Default|SpawnCharacter _asgm_master self Pawn%20Class))

(event Custom|OC_PlaceBlock
  (params (Color :type Linear%20Color%20Structure) (Transform :type Transform) (XFactor :type Integer) (YFactor :type Integer) (ZFactor :type Integer) (XPivot :type Integer) (YPivot :type Integer) (Top :type Integer))
  ;[1 1 1] Block Placement Mechanic
  ;;[1 1 1] Place Block
  (bind _returnvalue (Game|SpawnActorfromClass "/Game/Blueprints/Actors/BP_EditableBlock.BP_EditableBlock_C" Transform "AdjustIfPossibleButDontSpawnIfColliding" "MultiplyWithRoot" 0 0))
  (bind _returnvalue_2 (Rendering|Material|CreateDynamicMaterialInstance "/Game/Multiplayer/Widgets/ColorSelection/Color_box.Color_box" "None" "None" :!class /Script/Engine.KismetMaterialLibrary))
  (Rendering|Material|SetVectorParameterValue _returnvalue_2 "color" Color :!class /Script/Engine.MaterialInstanceDynamic)
  (Class|EditableBlock|SetMaterial _returnvalue _returnvalue_2)
  (Variables|/Game/Blueprints/Actors/BP_EditableBlock.BP_EditableBlock_C|SetPlaced _returnvalue true)
  (Default|SetSavedST _returnvalue Color Transform XFactor YFactor ZFactor XPivot YPivot Top)
  (Class|EditableBlock|GenerateBody _returnvalue XFactor YFactor ZFactor XPivot YPivot Top))

(event Custom|SR_SubmitChat
  (params (PlayerName :type Text) (ChatMessage :type Text))
  ;[0.05098 0.05098 0.05098] ChatBox
  (for _array_element (Variables|/Script/Engine.GameStateBase|GetPlayerArray (Game|GetGameState))
    (bind _aspc_master (Utilities|Casting|CastToPC_Master (Game|GetPlayerController _array_element)))
    (CallFunction|OCUpdateChat _aspc_master PlayerName ChatMessage)))

(event Custom|HandleOnClick
  (params (selection :type String))
  ;[1 1 1] Widget Selection
  (if (Utilities|Enum|Equal(Enum) selection "cube")
    (CallFunction|SetNewBlockParams 1 1 1 1 1 5)
    (Utilities|DeletePreviewBlock)
    (elif (Utilities|Enum|Equal(Enum) selection "cuboid")
      (CallFunction|SetNewBlockParams 1 3 1 1 3 5)
      (Utilities|DeletePreviewBlock)
      (else
        (CallFunction|SetNewBlockParams 2 2 2 1 1 1)
        (Utilities|DeletePreviewBlock)))))

(event Custom|SR_PlaceBlock
  (params (Color :type Linear%20Color%20Structure) (Transform :type Transform) (XFactor :type Integer) (YFactor :type Integer) (ZFactor :type Integer) (XPivot :type Integer) (YPivot :type Integer) (Top :type Integer))
  ;[1 1 1] Block Placement Mechanic
  ;;[1 1 1] Place Block
  (bind _asbp_game_instance (Utilities|GetLocalGameInstance))
  (Default|AddBlockData _asbp_game_instance (Utilities|MakeBlockST "/Game/Blueprints/Actors/BP_EditableBlock.BP_EditableBlock_C" Color Transform XFactor YFactor ZFactor XPivot YPivot Top))
  (for _array_element (Variables|/Script/Engine.GameStateBase|GetPlayerArray (Game|GetGameState))
    (bind _aspc_master (Utilities|Casting|CastToPC_Master (Game|GetPlayerController _array_element)))
    (CallFunction|OCPlaceBlock _aspc_master Color Transform XFactor YFactor ZFactor XPivot YPivot Top)))

(event Custom|SR_DeleteBlock
  (params (Start :type Vector) (End :type Vector) (Object%20Types :type Array%20of%20EObjectTypeQuery%20Enums :default "ObjectTypeQuery1") (Actors%20to%20Ignore :type Array%20of%20Actor%20Object%20References) (Initiating%20PC :type Player%20Controller%20Object%20Reference))
  ;[1 1 1] Block Placement Mechanic
  ;;[1 1 1] Delete Block
  (for _array_element (Variables|/Script/Engine.GameStateBase|GetPlayerArray (Game|GetGameState))
    (if (not (== (Game|GetPlayerController _array_element) Initiating%20PC))
      (bind _aspc_master (Utilities|Casting|CastToPC_Master (Game|GetPlayerController _array_element)))
      (CallFunction|OCDeleteBlock _aspc_master Start End Object%20Types Actors%20to%20Ignore))))

(event Custom|OC_DeleteBlock
  (params (Start :type Vector) (End :type Vector) (Object%20Types :type Array%20of%20EObjectTypeQuery%20Enums :default "ObjectTypeQuery1") (Actors%20to%20Ignore :type Array%20of%20Actor%20Object%20References))
  ;[1 1 1] Block Placement Mechanic
  ;;[1 1 1] Delete Block
  (Utilities|IsLocalPC
    (:true
      (bind (_outhit _returnvalue) (Collision|LineTraceForObjects Start End Object%20Types false Actors%20to%20Ignore "None"))
      (if _returnvalue
        (Development|PrintString (Utilities|GetDisplayName (.HitComponent (Collision|BreakHitResult _outhit))))
        (bind _asbp_editable_block (Utilities|Casting|CastToBP_EditableBlock (.HitActor (Collision|BreakHitResult _outhit))))
        (Default|SelfDestruct _asbp_editable_block (Networking|IsServer))))))

(event Custom|SR_LoadGame
  (params (Local_PC :type Player%20Controller%20Object%20Reference))
  ;[1 1 1] Load Game
  (bind _asbp_game_instance (Utilities|Casting|CastToBP_GameInstance (Game|GetGameInstance)))
  (bind _aspc_master (Utilities|Casting|CastToPC_Master Local_PC))
  (for _array_element (Variables|/Game/Multiplayer/SaveGame/BP_Saver.BP_Saver_C|GetBlocks (Variables|/Game/Multiplayer/BP_GameInstance.BP_GameInstance_C|GetBP_SaveRef _asbp_game_instance))
    (CallFunction|OCPlaceBlock _aspc_master (.color _array_element) (.transform _array_element) (.xfactor _array_element) (.yfactor _array_element) (.zfactor _array_element) (.xpivot _array_element) (.ypivot _array_element) (.top _array_element))))

(event EventBeginPlay
  (Utilities|IsLocalPC
    (:true
      (Utilities|FlowControl|Sequence
        (:then_0
          ;[1 1 1] Spawn PlayerPawn
          (bind _asbp_game_instance (Utilities|Casting|CastToBP_GameInstance (Game|GetGameInstance)))
          (bind _class (Utilities|AsyncLoadClassAsset (.CharacterBP (Utilities|Struct|BreakCharacters_Struct (Variables|/Game/Multiplayer/BP_GameInstance.BP_GameInstance_C|GetPlayer _asbp_game_instance))))
            (:Completed
              (bind _aspawn (Utilities|Casting|CastToPawnClass _class))
              (bind _output_get (Variables|Default|SetCharacter_Selection _aspawn))
              (CallFunction|SRSpawnPlayer _output_get)
              (Input|SetInputModeGameOnly self false))))
        (:then_1
          ;[1 1 1] Load Game
          (CallFunction|SRLoadGame self))
        (:then_2
          ;[0.05098 0.05098 0.05098] ChatBox
          (bind _returnvalue (UserInterface|CreateWidget "/Game/Multiplayer/Widgets/ChatBox/WB_ChatPanel.WB_ChatPanel_C" self))
          (bind _output_get_2 (Variables|Default|SetWB_ChatPanel _returnvalue))
          (UserInterface|Viewport|AddtoViewport _output_get_2 0))
        (:then_3
          ;[1 1 1] ColorPicker Widget
          (bind _returnvalue_2 (UserInterface|CreateWidget "/Game/Multiplayer/Widgets/ColorSelection/Widget_ColorPicker.Widget_ColorPicker_C"))
          (bind _output_get_3 (Variables|Default|SetWB_ColorPicker _returnvalue_2))
          (UserInterface|Viewport|AddtoViewport _output_get_3 0)
          (Widget|SetVisibility _output_get_3 "Hidden"))
        (:then_4
          ;[1 1 1] Widget Selection
          (bind _returnvalue_3 (UserInterface|CreateWidget "/Game/Multiplayer/Widgets/BoxSelection/WB_boxselection.WB_boxselection_C"))
          (bind _output_get_4 (Variables|Default|SetBoxSel _returnvalue_3))
          (UserInterface|Viewport|AddtoViewport _output_get_4 0)
          (Widget|SetVisibility _output_get_4 "Hidden"))
        (:then_5
          ;[1 1 1] Widget Selection
          (bind _returnvalue_4 (UserInterface|CreateWidget "/Game/Multiplayer/Widgets/BoxDesign/BlockDesign.BlockDesign_C"))
          (bind _output_get_5 (Variables|Default|SetBoxDes _returnvalue_4))
          (UserInterface|Viewport|AddtoViewport _output_get_5 0)
          (Widget|SetVisibility _output_get_5 "Hidden"))))))

(event EventTick
  (params (DeltaSeconds :type Float%20%28single-precision%29))
  ;[1 1 1] Block Placement Mechanic
  ;;[1 1 1] Preview Block
  (if (Pawn|IsLocalPlayerController)
    (Utilities|FlowControl|Sequence
      (:then_0
        ;;;[1 1 1] Get mouse hit position
        (bind _outputpin (Utilities|LineHitIgnore))
        (bind (_outhit _returnvalue) (Collision|LineTraceForObjects (stale _start) (stale _end) (Utilities|Array|MakeArray "ObjectTypeQuery1" "ObjectTypeQuery2" "ObjectTypeQuery4") false _outputpin "None"))
        (if _returnvalue
          (Utilities|IsValid (.HitComponent (Collision|BreakHitResult _outhit))
            (:Is%20Valid
              (bind _asstud (Utilities|Casting|CastToStud (.HitComponent (Collision|BreakHitResult _outhit)))
                (:then
                  (Variables|Default|SetMouse%20On%20Stud true)
                  (bind _output_get (Variables|Default|SetAs%20Stud _asstud))
                  (bind _rotation (CallFunction|CalculateRotation (.HitActor (Collision|BreakHitResult _outhit)) (Math|Vector|GetUpVector _output_get)))
                  (Variables|Default|SetPreview%20Transform (Math|Transform|MakeTransform (Transformation|GetWorldLocation _output_get) _rotation)))
                (:CastFailed
                  (Variables|Default|SetMouse%20On%20Stud false :!label _label))))
            (:Is%20Not%20Valid
              (goto _label)))
          (else
            (goto _label))))
      (:then_1
        ;;;[1 1 1] Check if mouse over something
        (if (Variables|Default|GetMouse%20On%20Stud)
          ;;;[1 1 1] Check if there is already a Preview Block
          (if (Utilities|IsValid (Variables|Default|GetPreview%20Block))
            ;;;[1 1 1] Set Preview Block at mouse position
            (Transformation|SetActorTransform (Variables|Default|GetPreview%20Block) (Variables|Default|GetPreview%20Transform))
            (else
              ;;;[1 1 1] Create EditableBlock to show as Preview Block
              (bind _returnvalue_2 (Game|SpawnActorfromClass "/Game/Blueprints/Actors/BP_EditableBlock.BP_EditableBlock_C" (Math|Transform|MakeTransform "0.000000,0.000000,-1000.000000" "0, 0, 0" "1.000000,1.000000,1.000000") "Undefined" "MultiplyWithRoot" 0 0))
              (bind _color (Default|ChangeBoxColor (Variables|Default|GetWB_ColorPicker)))
              (bind _returnvalue_3 (Rendering|Material|CreateDynamicMaterialInstance "/Game/Multiplayer/Widgets/ColorSelection/Color_box.Color_box" "None" "None" :!class /Script/Engine.KismetMaterialLibrary))
              (Rendering|Material|SetVectorParameterValue _returnvalue_3 "color" _color :!class /Script/Engine.MaterialInstanceDynamic)
              (Class|EditableBlock|SetMaterial _returnvalue_2 _returnvalue_3)
              (Collision|SetActorEnableCollision _returnvalue_2 false)
              (Variables|Default|SetPreview%20Block _returnvalue_2)
              (Class|EditableBlock|GenerateBody _returnvalue_2 (Variables|Default|GetXFactor) (Variables|Default|GetYFactor) (Variables|Default|GetZFactor) (Variables|Default|GetXPivot) (Variables|Default|GetYPivot) (Variables|Default|GetTop))))
          (else
            ;;;[1 1 1] Delete Preview Block if not hovering over something
            (Utilities|DeletePreviewBlock)))))))

(event Input|MouseEvents|LeftMouseButton
  (params (Key :type Key%20Structure :default "None"))
  ;[1 1 1] Block Placement Mechanic
  ;;[1 1 1] Place Block
  (:Pressed
    (Utilities|IsLocalPC
      (:true
        (if (Variables|Default|GetMouse%20On%20Stud)
          (bind _color (Default|ChangeBoxColor (Variables|Default|GetWB_ColorPicker)))
          (CallFunction|SRPlaceBlock _color (Variables|Default|GetPreview%20Transform) (Variables|Default|GetXFactor) (Variables|Default|GetYFactor) (Variables|Default|GetZFactor) (Variables|Default|GetXPivot) (Variables|Default|GetYPivot) (Variables|Default|GetTop)))))))

(event Input|MouseEvents|RightMouseButton
  (params (Key :type Key%20Structure :default "None"))
  (bind _array (Utilities|Array|MakeArray "ObjectTypeQuery1" "ObjectTypeQuery2" "ObjectTypeQuery4"))
  ;[1 1 1] Block Placement Mechanic
  ;;[1 1 1] Delete Block
  (:Pressed
    (Utilities|IsLocalPC
      (:true
        (bind _outputpin (Utilities|LineHitIgnore))
        (CallFunction|OCDeleteBlock (stale _start) (stale _end) _array _outputpin) ; Need to perform local delete first; otherwise mouse line wont find the right object in the initiating client
        (CallFunction|SRDeleteBlock (stale _start) (stale _end) _array _outputpin self)))))

(event Input|KeyboardEvents|Escape
  (params (Key :type Key%20Structure :default "None"))
  ;[0.05098 0.05098 0.05098] Open Pause Menu
  (:Pressed
    (bind _wb_pausemenu (Variables|Default|GetWB_PauseMenu)
      (:then
        (if (not (UserInterface|Viewport|IsinViewport _wb_pausemenu))
          (bind _returnvalue (UserInterface|CreateWidget "/Game/Multiplayer/Widgets/PauseMenu/WB_PauseMenu.WB_PauseMenu_C" self :!label _label))
          (bind _output_get (Variables|Default|SetWB_PauseMenu _returnvalue))
          (UserInterface|Viewport|AddtoViewport _output_get 0)
          (Input|SetInputModeGameandUI self (Variables|Default|GetWB_PauseMenu) "DoNotLock" true false)
          (Variables|Default|SetbShowMouseCursor true)))
      (:else
        (goto _label)))))

(event Input|KeyboardEvents|P
  (params (Key :type Key%20Structure :default "None"))
  (bind _self self)
  ;[1 1 1] ColorPicker Widget
  (:Pressed
    (bind _wb_colorpicker (Variables|Default|GetWB_ColorPicker)
      (:then
        (if (Utilities|Enum|Equal(Enum) (Widget|GetVisibility _wb_colorpicker) "Hidden")
          (Widget|SetVisibility _wb_colorpicker "Visible")
          (Input|SetInputModeGameandUI _self 0 "DoNotLock" true false)
          (Variables|/Script/Engine.PlayerController|SetbShowMouseCursor _self true)
          (else
            (Widget|SetVisibility _wb_colorpicker "Hidden")
            (Input|SetInputModeGameandUI _self 0 "DoNotLock" true false)
            (Variables|/Script/Engine.PlayerController|SetbShowMouseCursor _self true))))
      (:else))))

(event Input|KeyboardEvents|Enter
  (params (Key :type Key%20Structure :default "None"))
  ;[0.05098 0.05098 0.05098] ChatBox
  (:Pressed
    (bind _wb_chatpanel (Variables|Default|GetWB_ChatPanel)
      (:then
        (Widget|SetKeyboardFocus (Variables|/Game/Multiplayer/Widgets/ChatBox/WB_ChatPanel.WB_ChatPanel_C|GetChatInputBox _wb_chatpanel)))
      (:else))))

(event Input|MouseEvents|MouseWheelUp
  (params (Key :type Key%20Structure :default "None"))
  ;[0.05098 0.05098 0.05098] ChatBox
  (:Pressed
    (Default|Scroll (Variables|Default|GetWB_ChatPanel) true)))

(event Input|MouseEvents|MouseWheelDown
  (params (Key :type Key%20Structure :default "None"))
  ;[0.05098 0.05098 0.05098] ChatBox
  (:Pressed
    (Default|Scroll (Variables|Default|GetWB_ChatPanel) false)))

(event Input|KeyboardEvents|B
  (params (Key :type Key%20Structure :default "None"))
  ;[1 1 1] Spawn PlayerPawn
  ;;[1 1 1] Toggle between Spectator and Character
  (:Pressed
    (Utilities|IsLocalPC
      (:true
        (Utilities|FlowControl|FlipFlop
          (:A
            (CallFunction|SRSpawnPlayer "/Script/Engine.SpectatorPawn"))
          (:B
            (CallFunction|SRSpawnPlayer (Variables|Default|GetCharacter_Selection))))))))

(event Input|KeyboardEvents|R
  (params (Key :type Key%20Structure :default "None"))
  ;[1 1 1] Block Placement Mechanic
  ;;[1 1 1] Block Rotation
  (:Pressed
    (Variables|Default|SetRotation (Math|Rotator|MakeRotator 0.0 0.0 (Math|Float|%(Float) (+ 9e+01 (.yaw (Variables|Default|GetRotation))) 3.6e+02)))))

(event Input|KeyboardEvents|V
  (params (Key :type Key%20Structure :default "None"))
  ;[1 1 1] Experiment block for flying movement (There is a bug that is not fixed; Do not use)
)

(event Input|KeyboardEvents|L
  (params (Key :type Key%20Structure :default "None"))
  (bind _self self)
  (bind _boxsel (Variables|Default|GetBoxSel))
  ;[1 1 1] Widget Selection
  (:Pressed
    (if (Utilities|Enum|Equal(Enum) (Widget|GetVisibility _boxsel) "Hidden")
      (Widget|SetVisibility _boxsel "Visible")
      (Input|SetInputModeGameandUI _self 0 "DoNotLock" true false)
      (Variables|/Script/Engine.PlayerController|SetbShowMouseCursor _self true)
      (EventDispatchers|BindEventtoOnClick _boxsel (delegate Custom|HandleOnClick))
      (else
        (Widget|SetVisibility _boxsel "Hidden")
        (Input|SetInputModeGameandUI _self 0 "DoNotLock" true false)
        (Variables|/Script/Engine.PlayerController|SetbShowMouseCursor _self true)))))

(event Input|KeyboardEvents|F
  (params (Key :type Key%20Structure :default "None"))
  (bind _self self)
  (bind _boxdes (Variables|Default|GetBoxDes))
  ;[1 1 1] Widget Selection
  (:Pressed
    (if (Utilities|Enum|Equal(Enum) (Widget|GetVisibility _boxdes) "Hidden")
      (Widget|SetVisibility _boxdes "Visible")
      (Input|SetInputModeGameandUI _self 0 "DoNotLock" true false)
      (Variables|/Script/Engine.PlayerController|SetbShowMouseCursor _self true)
      (else
        (Widget|SetVisibility _boxdes "Hidden")
        (Input|SetInputModeGameandUI _self 0 "DoNotLock" true false)
        (Variables|/Script/Engine.PlayerController|SetbShowMouseCursor _self true)
        (bind _userinput (Default|ReturnMyValues _boxdes))
        (CallFunction|SetNewBlockParams (.Xmultiplier (Utilities|Struct|BreakInputStruct _userinput)) (.Ymultiplier (Utilities|Struct|BreakInputStruct _userinput)) (.Zmultiplier (Utilities|Struct|BreakInputStruct _userinput)) (.Pivotx (Utilities|Struct|BreakInputStruct _userinput)) (.Pivoty (Utilities|Struct|BreakInputStruct _userinput)) (.TopFace (Utilities|Struct|BreakInputStruct _userinput)))
        (Utilities|DeletePreviewBlock)))))

(fn ConstructionScript)

(fn CalculateRotation
  (params (Actor :type Actor%20Object%20Reference) (Normal :type Vector))
  (bind _returnvalue (Transformation|GetActorForwardVector Actor))
  (bind _returnvalue_2 (Math|Vector|ProjectVectorontoPlane _returnvalue Normal))
  (if (Math|Vector|VectorIsNearlyZero _returnvalue_2)
    (return (Math|Rotator|MakeRotfromZX Normal (Math|Vector|RotateVectorAroundAxis (Math|Vector|ProjectVectorontoPlane (Transformation|GetActorUpVector Actor) Normal) (.yaw (Variables|Default|GetRotation)) Normal)))
    (else
      (return (Math|Rotator|MakeRotfromZX Normal (Math|Vector|RotateVectorAroundAxis _returnvalue_2 (.yaw (Variables|Default|GetRotation)) Normal))))))

(fn SetNewBlockParams
  (params (XFactor :type Integer) (YFactor :type Integer) (ZFactor :type Integer) (XPivot :type Integer) (YPivot :type Integer) (Top :type Integer))
  (Variables|Default|SetXFactor XFactor)
  (Variables|Default|SetYFactor YFactor)
  (Variables|Default|SetZFactor ZFactor)
  (Variables|Default|SetXPivot XPivot)
  (Variables|Default|SetYPivot YPivot)
  (Variables|Default|SetTop Top)
  (return))