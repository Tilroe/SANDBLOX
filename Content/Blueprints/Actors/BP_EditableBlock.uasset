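; BP_EditableBlock is a block actor that pulses in size until it is marked as placed.
; The construction script calls GenerateBody to build the block.
; Tick accumulates elapsed time and, while Placed is false, drives a uniform sine-wave scale oscillation around normal size.
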(event `self.ReceiveTick`
  (params (DeltaSeconds :type "Float (single-precision)"))
  (bind _output_get (set `self.Time` (+ DeltaSeconds (`self.Time`))))
  (if (not (`self.Placed`))
    (`self.SetActorScale3D` (`KismetMathLibrary.Conv_DoubleToVector` (+ (* (`KismetMathLibrary.Sin` (* _output_get 3.0)) 0.1) 1.0)))))

(fn `UserConstructionScript`
  (`self.GenerateBody`))