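; Player pawn for a block-building mode that places and deletes editable blocks under the mouse cursor.
; Each tick traces the mouse ray to move, spawn or remove a preview block; left click places a copy, right click destroys non-ground hits.
; Number keys swap the vertex set used to generate block bodies.
; R steps yaw by 90 degrees, applied around the hit normal to the hit actor's projected forward vector.
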(event `Key|LeftMouseButton`
  (params (Key :type "Key Structure"))
  (bind (_start _end) (`self.Mouse Line`))
  ;[1 1 1] Place Block
  (:`Pressed`
    (bind (_outhit _returnvalue) (`KismetSystemLibrary.LineTraceSingleForObjects` _start _end (`|MakeArray` "ObjectTypeQuery1" "ObjectTypeQuery2" "ObjectTypeQuery4" :!type "EObjectTypeQuery Enum") false (`|MakeArray` (`self.Preview Block`))))
    (if _returnvalue
      (bind (_bblockinghit _binitialoverlap _time _distance _location _impactpoint _normal _impactnormal _physmat _hitactor) (`GameplayStatics.BreakHitResult` _outhit))
      (bind _returnvalue_2 (`|SpawnActorFromClass` "/Game/Blueprints/Actors/BP_EditableBlock.BP_EditableBlock_C" (`KismetMathLibrary.MakeTransform` _location (`self.Calculate Rotation` _normal (0.0 0.0 0.0) _hitactor)) "AdjustIfPossibleButDontSpawnIfColliding" "MultiplyWithRoot" null null))
      (`EditableBlock.SetVertices` _returnvalue_2 (`self.Vertices`))
      (set `/Game/Blueprints/Actors/BP_EditableBlock.Placed` true _returnvalue_2)
      (`EditableBlock.GenerateBody` _returnvalue_2))))

(event `Key|RightMouseButton`
  (params (Key :type "Key Structure"))
  (bind (_start _end) (`self.Mouse Line`))
  ;[1 1 1] Delete Block
  (:`Pressed`
    (bind _outactors (`GameplayStatics.GetAllActorsWithTag` "Ground"))
    (`KismetArrayLibrary.Array_Add` _outactors (`self.Preview Block`))
    (bind (_outhit _returnvalue) (`KismetSystemLibrary.LineTraceSingleForObjects` _start _end (`|MakeArray` "ObjectTypeQuery1" "ObjectTypeQuery2" "ObjectTypeQuery4" :!type "EObjectTypeQuery Enum") false _outactors))
    (if _returnvalue
      (`self.K2_DestroyActor` (`.HitActor` (`GameplayStatics.BreakHitResult` _outhit))))))

(event `self.ReceiveTick`
  (params (DeltaSeconds :type "Float (single-precision)"))
  (bind (_start _end) (`self.Mouse Line`))
  (`|ExecutionSequence`
    (:`then_0`
      ;[1 1 1] Get mouse hit position
      (bind (_outhit _returnvalue) (`KismetSystemLibrary.LineTraceSingleForObjects` _start _end (`|MakeArray` "ObjectTypeQuery1" "ObjectTypeQuery2" "ObjectTypeQuery4" :!type "EObjectTypeQuery Enum") false (`|MakeArray` (`self.Preview Block`)))))
    (:`then_1`
      ;[1 1 1] Check if mouse over something
      (if _returnvalue
        ;[1 1 1] Check if there is already a Preview Block
        (if (`KismetSystemLibrary.IsValid` (`self.Preview Block`))
          (bind (_bblockinghit _binitialoverlap _time _distance _location _impactpoint _normal _impactnormal _physmat _hitactor) (`GameplayStatics.BreakHitResult` _outhit))
          (bind _rotation (`self.Calculate Rotation` _normal _location _hitactor))
          ;[1 1 1] Set Preview Block at mouse position
          (`self.K2_SetActorTransform` (`self.Preview Block`) (`KismetMathLibrary.MakeTransform` _location _rotation) false false)
          (`KismetSystemLibrary.DrawDebugCoordinateSystem` _location _rotation 50.0 0.0 1.0)
          (else
            ;[1 1 1] Create EditableBlock to show as Preview Block
            (bind _returnvalue_2 (`|SpawnActorFromClass` "/Game/Blueprints/Actors/BP_EditableBlock.BP_EditableBlock_C" (`KismetMathLibrary.MakeTransform` (0.0 0.0 0.0)) "Undefined" "MultiplyWithRoot" null null))
            (`EditableBlock.SetVertices` _returnvalue_2 (`self.Vertices`))
            (set `self.Preview Block` _returnvalue_2)
            (`EditableBlock.GenerateBody` _returnvalue_2)))
        (else
          ;[1 1 1] Delete Preview Block if not hovering over something
          (`self.Delete Preview Block`))))))

(event `Key|One`
  (params (Key :type "Key Structure"))
  (:`Pressed`
    (set `self.Vertices` (`|MakeArray` (-40.0 -20.0 0.0) (-40.0 20.0 0.0) (40.0 -20.0 0.0) (40.0 20.0 0.0) (-40.0 -20.0 20.0) (-40.0 20.0 20.0) (40.0 -20.0 20.0) (40.0 20.0 20.0) :!type "Vector Structure"))
    (`self.Delete Preview Block`)))

(event `Key|R`
  (params (Key :type "Key Structure"))
  (bind (_rotation_roll _rotation_pitch _rotation_yaw) (`KismetMathLibrary.BreakRotator` (`self.Rotation`)))
  (:`Pressed`
    (bind _output_get (set `self.Rotation` (`KismetMathLibrary.MakeRotator` 0.0 0.0 (mod (+ 90.0 _rotation_yaw) 360.0))))
    (`KismetSystemLibrary.PrintString` (`KismetStringLibrary.Conv_RotatorToString` _output_get))))

(event `Key|Two`
  (params (Key :type "Key Structure"))
  (:`Pressed`
    (set `self.Vertices` (`|MakeArray` (-20.0 -20.0 0.0) (-20.0 20.0 0.0) (20.0 -20.0 0.0) (20.0 20.0 0.0) (-20.0 -20.0 20.0) (-20.0 20.0 20.0) (20.0 -20.0 20.0) (20.0 20.0 20.0) :!type "Vector Structure"))
    (`self.Delete Preview Block`)))

(event `Key|Three`
  (params (Key :type "Key Structure"))
  (:`Pressed`
    (set `self.Vertices` (`|MakeArray` (-20.0 -20.0 0.0) (-20.0 20.0 0.0) (20.0 -20.0 0.0) (20.0 20.0 0.0) (-20.0 -20.0 20.0) (-20.0 20.0 20.0) :!type "Vector Structure"))
    (`self.Delete Preview Block`)))

(fn `UserConstructionScript`)