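; BP_EditableBlock1 is an actor that builds a procedural tetrahedron in a Dynamic Mesh Component as a base for vertex editing.
; The construction script resets the mesh, adds four hard-coded vertices through Geometry Script and joins their returned array indices into four triangles.
; DeleteVertex wraps vertex removal but has no target mesh wired and no caller in this graph.
; RandomVertex is unfinished, and BeginPlay only fetches the mesh.
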(event `self.ReceiveBeginPlay`
  (`BaseDynamicMeshComponent.GetDynamicMesh` (`self.DynamicMeshComponent`)))

(fn `Delete Vertex`
  (params (`Vertex ID` :type Integer))
  (`GeometryScriptLibrary_MeshBasicEditFunctions.DeleteVertexFromMesh` null `Vertex ID`))

(fn `UserConstructionScript`
  (locals (`First Vertices` :type "Array of Vector Structure") (`Dynamic Mesh Reference` :type "DynamicMesh Object Reference"))
  (bind _dynamic_mesh_reference (`local.Dynamic Mesh Reference`))
  (bind _returnvalue (`BaseDynamicMeshComponent.GetDynamicMesh` (`self.DynamicMeshComponent`)))
  (bind _returnvalue_2 (`DynamicMesh.Reset` _returnvalue))
  (set `local.Dynamic Mesh Reference` _returnvalue_2)
  (bind _output_get (set `local.First Vertices` (`|MakeArray`)))
  (bind _returnvalue_3 (`KismetArrayLibrary.Array_Add` _output_get (`KismetMathLibrary.Conv_IntVectorToVector` (make `IntVector` 0 100))))
  (bind _returnvalue_4 (`KismetArrayLibrary.Array_Add` _output_get (`KismetMathLibrary.Conv_IntVectorToVector` (make `IntVector` -50 -50))))
  (bind _returnvalue_5 (`KismetArrayLibrary.Array_Add` _output_get (`KismetMathLibrary.Conv_IntVectorToVector` (make `IntVector` 50 -50))))
  (bind _returnvalue_6 (`KismetArrayLibrary.Array_Add` _output_get (`KismetMathLibrary.Conv_IntVectorToVector` (make `IntVector` 0 0 50))))
  (bind _vectorlist (`GeometryScriptLibrary_ListUtilityFunctions.ConvertArrayToVectorList` (`local.First Vertices`)))
  (`GeometryScriptLibrary_MeshBasicEditFunctions.AddVerticesToMesh` (`local.Dynamic Mesh Reference`) _vectorlist)
  (`GeometryScriptLibrary_MeshBasicEditFunctions.AddTriangleToMesh` _dynamic_mesh_reference (make `IntVector` _returnvalue_3 _returnvalue_4 _returnvalue_5) 0 false null)
  (`GeometryScriptLibrary_MeshBasicEditFunctions.AddTriangleToMesh` _dynamic_mesh_reference (make `IntVector` _returnvalue_3 _returnvalue_6 _returnvalue_4) 0 false null)
  (`GeometryScriptLibrary_MeshBasicEditFunctions.AddTriangleToMesh` _dynamic_mesh_reference (make `IntVector` _returnvalue_3 _returnvalue_5 _returnvalue_6) 0 false null)
  (`GeometryScriptLibrary_MeshBasicEditFunctions.AddTriangleToMesh` _dynamic_mesh_reference (make `IntVector` _returnvalue_4 _returnvalue_6 _returnvalue_5) 0 false null))