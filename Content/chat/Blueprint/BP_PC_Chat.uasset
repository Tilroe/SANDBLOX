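; Player controller that gives each player a multiplayer text chat.
; On begin play, the local controller creates and shows a WB_ChatPanel widget, and Enter puts keyboard focus on its input box.
; SR_SubmitChat relays a name and message to every chat controller in the game state's PlayerArray.
; OC_UpdateChat passes them to that player's panel, with the prefixes suggesting a server-to-owning-client RPC fan-out.
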(event `self.ReceiveBeginPlay`
  (if (`self.IsLocalPlayerController`)
    (bind _returnvalue (`|CreateWidget` "/Game/chat/Widgets/WB_ChatPanel.WB_ChatPanel_C" self))
    (bind _output_get (set `self.WB_ChatPanel` _returnvalue))
    (`UserWidget.AddToViewport` _output_get 0)))

(event `Key|Enter`
  (params (Key :type "Key Structure"))
  (:`Pressed`
    (bind _wb_chatpanel (`self.WB_ChatPanel`)
      (:`then`
        (`Widget.SetKeyboardFocus` (`/Game/chat/Widgets/WB_ChatPanel.ChatInputBox` _wb_chatpanel)))
      (:`else`))))

(event `SR_SubmitChat`
  (params (PlayerName :type Text) (ChatMessage :type Text))
  (for _array_element (`GameStateBase.PlayerArray` (`GameplayStatics.GetGameState`))
    (bind _asbp_pc_chat (cast `/Game/chat/Blueprint/BP_PC_Chat` (`PlayerState.GetPlayerController` _array_element)))
    (`self.OC_UpdateChat` _asbp_pc_chat PlayerName ChatMessage)))

(event `OC_UpdateChat`
  (params (PlayerName :type Text) (ChatMessage :type Text))
  (bind _wb_chatpanel (`self.WB_ChatPanel`)
    (:`then`
      (`/Game/chat/Widgets/WB_ChatPanel.Update_chat` _wb_chatpanel PlayerName ChatMessage))
    (:`else`)))

(fn `UserConstructionScript`)